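; BP_DamagableActor is a prototype interactable actor that can take damage and be killed.
; On BeginPlay it binds handlers to its BPHealthComponent's took-damage and killed events.
; Taking damage only prints a debug string, while death plays a sound, destroys the actor and spawns a particle system at its location.
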(event `CustomEvent`
  (params (Damage :type "Float (double-precision)"))
  (`KismetSystemLibrary.PrintString` "owie"))

(event `self.ReceiveBeginPlay`
  (bind _bp_healthcomponent (`self.BP_HealthComponent`))
  (add `/Game/GamePrototyping/Components/BP_HealthComponent.OnKilled` _bp_healthcomponent (delegate `DIE`))
  (add `/Game/GamePrototyping/Components/BP_HealthComponent.OnTookDamage` _bp_healthcomponent (delegate `CustomEvent`)))

(event `DIE`
  (`GameplayStatics.SpawnSoundAtLocation` (`self.Death_SFX`) (`self.K2_GetActorLocation`) (struct) 1.0 1.0 0.0 null null)
  (`self.K2_DestroyActor`)
  (`NiagaraFunctionLibrary.SpawnSystemAtLocation` "/Game/GamePrototyping/Particles/Death_Particles.Death_Particles" (`self.K2_GetActorLocation`)))

(fn `UserConstructionScript`)