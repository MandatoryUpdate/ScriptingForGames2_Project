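; Player controller that sets up input and the HUD for the local player and handles leaving the game.
; On BeginPlay, for the local controller only, it adds the game's Enhanced Input mapping context and creates, stores and displays BP_HUD.
; The IA_LeaveGame action quits the game.
; GetCurrentMousePosition returns the screen-space cursor as a vector on the XZ plane, with Y zeroed, without converting it to world space.
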(event `self.ReceiveBeginPlay`
  (if (`self.IsLocalPlayerController`)
    (`|ExecutionSequence`
      (:`then_0`
        (`EnhancedInputSubsystemInterface.AddMappingContext` (subsystem `EnhancedInputLocalPlayerSubsystem`) "/Game/GamePrototyping/ActualGameCharacters/Input_Actions_And_Context/GameInput_MappingContext.GameInput_MappingContext" 0 (struct))
        (bind _returnvalue (`|CreateWidget` "/Game/GamePrototyping/ActualGameCharacters/BP_HUD.BP_HUD_C" self))
        (bind _output_get (set `self.PlayerHud` _returnvalue))
        (`UserWidget.AddToViewport` _output_get 0)))))

(event `EnhancedInput|/Game/GamePrototyping/ActualGameCharacters/Input_Actions_And_Context/IA_LeaveGame`
  (params (ActionValue :type Boolean) (ElapsedSeconds :type "Float (double-precision)") (TriggeredSeconds :type "Float (double-precision)") (InputAction :type "InputAction Object Reference" :default "/Game/GamePrototyping/ActualGameCharacters/Input_Actions_And_Context/IA_LeaveGame.IA_LeaveGame"))
  (:`Triggered`
    (`KismetSystemLibrary.QuitGame` null "Quit")))

(fn `GetCurrentMousePosition`
  (returns (MouseWorldPosition :type "Vector Structure"))
  (bind (_locationx _locationy _returnvalue) (`self.GetMousePosition`))
  (if _returnvalue
    (return (`KismetMathLibrary.MakeVector` _locationx 0.0 _locationy))))

(fn `UserConstructionScript`)