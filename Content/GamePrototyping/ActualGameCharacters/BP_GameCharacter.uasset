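; Player character that moves forward and back, fires at the mouse cursor, tracks scrap and quits the game when killed.
; On BeginPlay it spawns test weapons, attaches them to the head socket and stores them deactivated.
; Input fires, reloads or cycles weapons, refreshing the HUD on swap; the cycle wraps before the last entry.
; Aim deprojects the mouse onto a camera-facing plane, set at the character's horizontal distance from the camera.
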(event `self.ReceiveBeginPlay`
  (bind _asbp_game_controller (cast `/Game/GamePrototyping/ActualGameCharacters/BP_GameController` (`GameplayStatics.GetPlayerController` 0)))
  (`EnhancedInputSubsystemInterface.AddMappingContext` (pcsubsystem `EnhancedInputLocalPlayerSubsystem` _asbp_game_controller) "/Game/GamePrototyping/ActualGameCharacters/Input_Actions_And_Context/PlayerInputActionContext.PlayerInputActionContext" 0 (struct))
  (add `/Game/GamePrototyping/Components/BP_HealthComponent.OnKilled` (`self.BP_HealthComponent`) (delegate `OnKilled`))
  (for _array_element (`self.WeaponSpawner(ForTesting)`)
    (bind _returnvalue (`|SpawnActorFromClass` _array_element (`self.GetTransform`) "Undefined" "MultiplyWithRoot" null self))
    (bind _output_get (set `self.CurrentWeapon` _returnvalue))
    (`self.K2_AttachToActor` _output_get self "None" "KeepRelative" "KeepRelative" "KeepRelative" true)
    (`SceneComponent.K2_AttachToComponent` (`/Game/GamePrototyping/Guns/BP_Gun.Cube` _output_get) (`self.Mesh`) "head" "KeepRelative" "KeepRelative" "KeepRelative" true)
    (`/Game/GamePrototyping/Guns/BP_Gun.SetDeactivated` _output_get)
    (`KismetArrayLibrary.Array_AddUnique` (`self.CollectedWeapons`) _output_get)))

(event `OnKilled`
  (`KismetSystemLibrary.QuitGame` null "Quit"))

(event `EnhancedInput|/Game/GamePrototyping/ActualGameCharacters/Input_Actions_And_Context/IA_SwapWeapons`
  (params (ActionValue :type Boolean) (ElapsedSeconds :type "Float (double-precision)") (TriggeredSeconds :type "Float (double-precision)") (InputAction :type "InputAction Object Reference" :default "/Game/GamePrototyping/ActualGameCharacters/Input_Actions_And_Context/IA_SwapWeapons.IA_SwapWeapons"))
  (bind _currentweapon (`self.CurrentWeapon`))
  (bind _weaponlistposition (`self.WeaponListPosition`))
  (:`Started`
    (`/Engine/EditorBlueprintResources/StandardMacros.IsValid` _currentweapon
      (:`Is Valid`
        (`/Game/GamePrototyping/Guns/BP_Gun.SetDeactivated` _currentweapon)
        (`KismetArrayLibrary.Array_Set` (`self.CollectedWeapons`) (`KismetMathLibrary.FTrunc` (`self.WeaponListPosition`)) (`self.CurrentWeapon`))
        (`/Engine/EditorBlueprintResources/StandardMacros.IncrementFloat` _weaponlistposition
          (:`  `
            (if (not (< _weaponlistposition (- (`KismetArrayLibrary.Array_Length` (`self.CollectedWeapons`)) 1)))
              (set `self.WeaponListPosition` 0.0))
            (bind _output_get (set `self.CurrentWeapon` (`|GetArrayItem` (`self.CollectedWeapons`) (`KismetMathLibrary.FTrunc` (`self.WeaponListPosition`)))))
            (`/Game/GamePrototyping/Guns/BP_Gun.SetActive` _output_get)
            (bind _asbp_game_controller (cast `/Game/GamePrototyping/ActualGameCharacters/BP_GameController` (`GameplayStatics.GetPlayerController` 0)))
            (`/Game/GamePrototyping/HUD/BP_HUD.OnWeaponGainedOrChanged` (`/Game/GamePrototyping/ActualGameCharacters/BP_GameController.PlayerHud` _asbp_game_controller))))))))

(event `EnhancedInput|/Game/GamePrototyping/ActualGameCharacters/Input_Actions_And_Context/IA_MoveForward`
  (params (ActionValue :type Boolean) (ElapsedSeconds :type "Float (double-precision)") (TriggeredSeconds :type "Float (double-precision)") (InputAction :type "InputAction Object Reference" :default "/Game/GamePrototyping/ActualGameCharacters/Input_Actions_And_Context/IA_MoveForward.IA_MoveForward"))
  (:`Ongoing`
    (`self.AddMovementInput` (`self.GetActorForwardVector`) 1000.0)))

(event `EnhancedInput|/Game/GamePrototyping/ActualGameCharacters/Input_Actions_And_Context/IA_MoveBackward`
  (params (ActionValue :type Boolean) (ElapsedSeconds :type "Float (double-precision)") (TriggeredSeconds :type "Float (double-precision)") (InputAction :type "InputAction Object Reference" :default "/Game/GamePrototyping/ActualGameCharacters/Input_Actions_And_Context/IA_MoveBackward.IA_MoveBackward"))
  (:`Ongoing`
    (`self.AddMovementInput` (* (`self.GetActorForwardVector`) -1.0) 1000.0)))

(event `EnhancedInput|/Game/GamePrototyping/ActualGameCharacters/Input_Actions_And_Context/IA_Reload`
  (params (ActionValue :type Boolean) (ElapsedSeconds :type "Float (double-precision)") (TriggeredSeconds :type "Float (double-precision)") (InputAction :type "InputAction Object Reference" :default "/Game/GamePrototyping/ActualGameCharacters/Input_Actions_And_Context/IA_Reload.IA_Reload"))
  (:`Started`
    (`/Game/GamePrototyping/Guns/BP_Gun.Reload` (`self.CurrentWeapon`))))

(event `EnhancedInput|/Game/GamePrototyping/ActualGameCharacters/Input_Actions_And_Context/IA_Fire`
  (params (ActionValue :type Boolean) (ElapsedSeconds :type "Float (double-precision)") (TriggeredSeconds :type "Float (double-precision)") (InputAction :type "InputAction Object Reference" :default "/Game/GamePrototyping/ActualGameCharacters/Input_Actions_And_Context/IA_Fire.IA_Fire"))
  (bind _returnvalue (`self.K2_GetActorLocation`))
  (bind _directionalvector (`self.DirectionalVector`))
  (bind _currentweapon (`self.CurrentWeapon`))
  (bind _currentweapon_2 (`self.CurrentWeapon`))
  (:`Started`
    (`self.UpdateMousePosition`)
    (`/Engine/EditorBlueprintResources/StandardMacros.IsValid` _currentweapon_2
      (:`Is Valid`
        (bind _output_get (set `self.AimRotation` (`KismetMathLibrary.FindLookAtRotation` (+ (* 10.0 (`KismetMathLibrary.GetForwardVector` (`KismetMathLibrary.FindLookAtRotation` _returnvalue _directionalvector))) _returnvalue) _directionalvector)))
        (bind _returnvalue_2 (`KismetMathLibrary.MakeTransform` (`self.K2_GetActorLocation`) _output_get))
        (`/Game/GamePrototyping/Guns/BP_Gun.Fire` _currentweapon_2 _returnvalue_2))))
  (:`Ongoing`
    (`/Engine/EditorBlueprintResources/StandardMacros.IsValid` _currentweapon
      (:`Is Valid`
        (if (`/Game/GamePrototyping/Guns/BP_Gun.IsAuto` _currentweapon)
          (`/Game/GamePrototyping/Guns/BP_Gun.Fire` _currentweapon _returnvalue_2))))))

(event `EnhancedInput|/Game/Input/Actions/IA_MouseLook`
  (params (ActionValue :type "Vector2D Structure") (ElapsedSeconds :type "Float (double-precision)") (TriggeredSeconds :type "Float (double-precision)") (InputAction :type "InputAction Object Reference" :default "/Game/Input/Actions/IA_MouseLook.IA_MouseLook"))
  (:`Triggered`
    (`self.UpdateMousePosition`)))

(fn `ChangeScrap`
  (params (AmountChange :type "Float (double-precision)"))
  (set `self.ScrapCount` (+ (`self.ScrapCount`) AmountChange))
  (`self.ScrapChanged`))

(fn `UpdateMousePosition`
  (set `self.DirectionalVector` (+ (`PlayerCameraManager.GetCameraLocation` (`GameplayStatics.GetPlayerCameraManager` 0)) (* (/ (`KismetMathLibrary.VSize` (`KismetMathLibrary.MakeVector` (- (.x (`self.K2_GetActorLocation` self)) (.x (`PlayerCameraManager.GetCameraLocation` (`GameplayStatics.GetPlayerCameraManager` 0)))) (- (.y (`self.K2_GetActorLocation` self)) (.y (`PlayerCameraManager.GetCameraLocation` (`GameplayStatics.GetPlayerCameraManager` 0)))))) (`KismetMathLibrary.DegCos` (`KismetMathLibrary.DegAcos` (`KismetMathLibrary.Dot_VectorVector` (`KismetMathLibrary.GetForwardVector` (`PlayerCameraManager.GetCameraRotation` (`GameplayStatics.GetPlayerCameraManager` 0))) (`.WorldDirection` (`PlayerController.DeprojectMousePositionToWorld` (`GameplayStatics.GetPlayerController` 0))))))) (`.WorldDirection` (`PlayerController.DeprojectMousePositionToWorld` (`GameplayStatics.GetPlayerController` 0)))))))

(fn `UserConstructionScript`)