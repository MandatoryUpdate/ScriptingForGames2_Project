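; Reusable health component that tracks an actor's current health and reports damage, healing and death through event dispatchers.
; On BeginPlay it fills health to max and binds to the owner's OnTakeAnyDamage event.
; Damage is subtracted and clamped, then either fires OnKilled at zero or plays a hit sound and fires OnTookDamage, which is passed zero rather than the damage amount.
; Heal adds clamped health and fires OnHealed.
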(event `self.ReceiveBeginPlay`
  (set `self.Owner` (`self.GetOwner`))
  (set `self.CurrentHealth` (`self.MaxHealth`))
  (add `Actor.OnTakeAnyDamage` (`self.Owner`) (`|CreateDelegate` :!event `TookDamage`)))

(event `TookDamage`
  (params (DamagedActor :type "Actor Object Reference") (Damage :type "Float (single-precision)") (DamageType :type "DamageType Object Reference") (InstigatedBy :type "Controller Object Reference") (DamageCauser :type "Actor Object Reference"))
  (set `self.CurrentHealth` (`KismetMathLibrary.FClamp` (- (`self.CurrentHealth`) Damage) 0.0 (`self.MaxHealth`)))
  (if (<= (`self.CurrentHealth`) 0.0)
    (`self.OnKilled`)
    (else
      (`GameplayStatics.SpawnSoundAtLocation` (`self.Damage_SFX`) (`Actor.K2_GetActorLocation` (`self.GetOwner`)) (struct) 1.0 1.0 0.0 null null)
      (`self.OnTookDamage` 0.0))))

(fn `Heal`
  (params (Amount :type "Float (double-precision)"))
  (set `self.CurrentHealth` (`KismetMathLibrary.FClamp` (+ (`self.CurrentHealth`) Amount) 0.0 (`self.MaxHealth`)))
  (`self.OnHealed`))