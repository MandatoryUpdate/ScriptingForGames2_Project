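; BP_Gun is a gun actor with magazine and reserve ammo that can be shown or hidden as it is activated or deactivated.
; Fire spawns a bullet and sound, then launches the attached BP_GameCharacter opposite the shot as recoil.
; Semi-auto shots wait on a cooldown timer via CanFire, while auto fire skips that check.
; An empty magazine triggers a timed reload from reserve, and call events announce shots, reloads and ammo gains.
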(event `OnAmmoGained`
  (params (AmountAdded :type "Float (double-precision)"))
  (set `self.TotalAmmo` (+ (`self.TotalAmmo`) AmountAdded))
  (`self.GainedAmmo`))

(event `self.ReceiveBeginPlay`
  (set `self.CurrentAmmo` (`self.MagazineSize`)))

(event `Reload`
  (if (`self.ShouldReload?`)
    (if (not (<= (`self.TotalAmmo`) 0.0))
      (set `self.ShouldReload?` false)
      (set `self.CanFire` false)
      (`KismetSystemLibrary.PrintString` "Start Reload")
      (`KismetSystemLibrary.K2_SetTimerDelegate` (delegate `DoTheStuff`) (`self.ReloadTime`) false true))))

(event `DoTheStuff`
  (bind _totalammo (`self.TotalAmmo`))
  (bind _returnvalue (- (`self.MagazineSize`) (`self.CurrentAmmo`)))
  (if (< _totalammo (`self.MagazineSize`))
    (set `self.CurrentAmmo` _totalammo)
    (set `self.TotalAmmo` 0.0)
    (else
      (set `self.TotalAmmo` (`KismetMathLibrary.FClamp` (- _totalammo _returnvalue) 0.0 _totalammo))
      (set `self.CurrentAmmo` (+ _returnvalue (`self.CurrentAmmo`)))))
  (set `self.CanFire` true)
  (`KismetSystemLibrary.PrintString` (`KismetStringLibrary.Conv_DoubleToString` (`self.TotalAmmo`)))
  (set `self.ShouldReload?` true)
  (`self.Reloaded`))

(event `Fire`
  (params (BulletSpawnPosition :type "Transform Structure"))
  (bind _returnvalue (`self.GetAttachParentActor`))
  (if (> (`self.CurrentAmmo`) 0.0)
    (if (`self.IsAuto`)
      (set `self.CurrentAmmo` (`KismetMathLibrary.FClamp` (- (`self.CurrentAmmo`) 1.0) 0.0 (`self.MagazineSize`)) :!label _label)
      (`GameplayStatics.SpawnSoundAtLocation` "/Game/GamePrototyping/Sounds/Firing_SFX_Cue.Firing_SFX_Cue" (`self.K2_GetActorLocation`) (struct) 1.0 1.0 0.0 null null)
      (`|SpawnActorFromClass` (`self.BulletType`) BulletSpawnPosition "Undefined" "MultiplyWithRoot" self null)
      (`KismetSystemLibrary.K2_SetTimerDelegate` (delegate `CustomEvent`) (`self.CooldownTime`) false true)
      (`/Engine/EditorBlueprintResources/StandardMacros.IsValid` _returnvalue
        (:`Is Valid`
          (bind _asbp_game_character (cast `/Game/GamePrototyping/ActualGameCharacters/BP_GameCharacter` _returnvalue))
          (`Character.LaunchCharacter` _asbp_game_character (* (* (`KismetMathLibrary.GetForwardVector` (.rotation BulletSpawnPosition)) -1.0) (`self.Force`)) true true)
          (`self.Fired`)))
      (elif (`self.CanFire`)
        (set `self.CanFire` false)
        (goto _label)))
    (else
      (`self.Reload`))))

(event `CustomEvent`
  (set `self.CanFire` true))

(event `SetActive`
  (`self.SetActorHiddenInGame` false)
  (set `self.CanFire` true))

(event `SetDeactivated`
  (`self.SetActorHiddenInGame` true)
  (set `self.CanFire` false))

(fn `UserConstructionScript`)