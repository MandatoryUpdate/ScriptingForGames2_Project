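; Bullet actor for the prototype guns that damages what it hits and then destroys itself.
; An overlap on its sphere calls CalculateAndDealDamage, which ignores the first player's pawn and applies engine damage only to actors with a BP_HealthComponent.
; Any other overlap still spawns the Niagara hit particles at the bullet's location and destroys it.
; Leftover unreachable nodes hold an older self-check and TookDamage call.
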(event `self.Sphere1.OnComponentBeginOverlap`
  (params (OverlappedComponent :type "PrimitiveComponent Object Reference") (OtherActor :type "Actor Object Reference") (OtherComp :type "PrimitiveComponent Object Reference") (OtherBodyIndex :type Integer) (bFromSweep :type Boolean) (SweepResult :type "HitResult Structure (by ref)"))
  (`self.CalculateAndDealDamage` OtherActor OtherActor OtherActor OtherActor))

(fn `CalculateAndDealDamage`
  (params (self2 :type "Actor Object Reference") (B :type "Object Object Reference") (DamagedActor :type "Actor Object Reference") (A :type "Object Object Reference"))
  (if (!= (`GameplayStatics.GetPlayerPawn` 0) B)
    (`/Engine/EditorBlueprintResources/StandardMacros.IsValid` (`self.GetComponentByClass` self2 "/Game/GamePrototyping/Components/BP_HealthComponent.BP_HealthComponent_C")
      (:`Is Valid`
        (`GameplayStatics.ApplyDamage` DamagedActor (`self.Damage`) null self))
      (:`Is Not Valid`
        _))
    (`NiagaraFunctionLibrary.SpawnSystemAtLocation` "/Game/GamePrototyping/Particles/Bullet_Hit_Particles.Bullet_Hit_Particles" (`self.K2_GetActorLocation`))
    (`self.K2_DestroyActor`)))

(fn `UserConstructionScript`)