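; BP_Scrap_Gun is a gun that fires bullets using its attached game character's scrap as ammo.
; Fire casts the attach parent to BP_GameCharacter, then, if scrap remains and CanFire is set on a non-auto gun, plays a sound, spawns BP_Bullet and deducts scrap.
; A cooldown timer then sets CanFire true, though nothing here clears it.
; Reload is empty and automatic fire has no logic.
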(event `self.ReceiveBeginPlay`)

(event `self.Fire`
  (params (BulletSpawnPosition :type "Transform Structure"))
  (bind _asbp_game_character (cast `/Game/GamePrototyping/ActualGameCharacters/BP_GameCharacter` (`self.GetAttachParentActor`)))
  (if (> (`/Game/GamePrototyping/ActualGameCharacters/BP_GameCharacter.ScrapCount` _asbp_game_character) 0.0)
    (if (`self.IsAuto`)
      _
      (elif (`self.CanFire`)
        (`GameplayStatics.SpawnSoundAtLocation` "/Game/GamePrototyping/Sounds/Firing_SFX_Cue.Firing_SFX_Cue" (`self.K2_GetActorLocation`) (struct) 1.0 1.0 0.0 null null)
        (`|SpawnActorFromClass` "/Game/GamePrototyping/Guns/BP_Bullet.BP_Bullet_C" BulletSpawnPosition "Undefined" "MultiplyWithRoot" null null)
        (`/Game/GamePrototyping/ActualGameCharacters/BP_GameCharacter.ChangeScrap` _asbp_game_character -1.0)
        (`KismetSystemLibrary.K2_SetTimerDelegate` (delegate `CustomEvent_1`) (`self.CooldownTime`) false true)))))

(event `self.Reload`)

(event `CustomEvent_1`
  (set `self.CanFire` true))

(fn `NewFunction`)

(fn `UserConstructionScript`
  (bind _returnvalue (`self.GetAttachParentActor`))
  (if (== _returnvalue "/Game/GamePrototyping/ActualGameCharacters/BP_GameCharacter.BP_GameCharacter")
    (set `self.NewVar` _returnvalue)))