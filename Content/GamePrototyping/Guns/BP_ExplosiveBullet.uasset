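; BP_ExplosiveBullet is a bullet actor that explodes when its sphere component overlaps any actor other than the player pawn.
; The overlap calls CalculateAndDealDamage, which applies radial damage with falloff scaled from the Damage and DamageRadius variables, using a custom trace channel for damage prevention.
; It then prints the result, draws a long-lived debug sphere at the blast radius and destroys itself.
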(event `self.Sphere1.OnComponentBeginOverlap`
  (params (OverlappedComponent :type "PrimitiveComponent Object Reference") (OtherActor :type "Actor Object Reference") (OtherComp :type "PrimitiveComponent Object Reference") (OtherBodyIndex :type Integer) (bFromSweep :type Boolean) (SweepResult :type "HitResult Structure (by ref)"))
  (`self.CalculateAndDealDamage` OtherActor OtherActor OtherActor OtherActor))

(fn `CalculateAndDealDamage`
  (params (self2 :type "Actor Object Reference") (B :type "Object Object Reference") (DamagedActor :type "Actor Object Reference") (A :type "Object Object Reference"))
  (bind _returnvalue (`self.K2_GetActorLocation`))
  (bind _damageradius (`self.DamageRadius`))
  (bind _damage (`self.Damage`))
  (if (!= DamagedActor (`GameplayStatics.GetPlayerPawn` 0))
    (bind _returnvalue_2 (`GameplayStatics.ApplyRadialDamageWithFalloff` :`BaseDamage` _damage :`MinimumDamage` (/ _damage 2.0) :`Origin` _returnvalue :`DamageInnerRadius` (/ _damageradius 2.0) :`DamageOuterRadius` _damageradius :`DamageFalloff` 0.2 :`DamageCauser` self :`InstigatedByController` null :`DamagePreventionChannel` "ECC_GameTraceChannel1"))
    (`KismetSystemLibrary.PrintString` (`KismetStringLibrary.Conv_BoolToString` _returnvalue_2))
    (`KismetSystemLibrary.DrawDebugSphere` _returnvalue _damageradius 12 (struct :`R` 1.0 :`G` 1.0 :`B` 1.0 :`A` 1.0) 400.0)
    (`self.K2_DestroyActor`)))

(fn `UserConstructionScript`
  (`parent.UserConstructionScript`))